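; Game mode for a dungeon that moves the player between randomly chosen trap rooms.
; On BeginPlay it gathers all room managers and treats the first as the current room.
; SpawnNextRoom clears the current room's traps, spawns traps in a random room and teleports the player to its spawn point.
; SpawnTrap fills given transforms with floor pieces, letting one random slot become a random trap by weighted chance.
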(event `self.ReceiveBeginPlay`
  (bind _outactors (`GameplayStatics.GetAllActorsOfClass` "/Game/Dungeon/Blueprints/Utils/BP_RoomManager.BP_RoomManager_C"))
  (bind _output_get (set `self.TrapRooms` _outactors))
  (set `self.LastTrapRoom` (`|GetArrayItem` _output_get)))

(event `SpawnNextRoom`
  (`/Game/Dungeon/Blueprints/Utils/BP_RoomManager.Destroy Traps` (`self.LastTrapRoom`))
  (bind _output_get (set `self.LastTrapRoom` (`KismetArrayLibrary.Array_Random` (`self.TrapRooms`))))
  (`/Game/Dungeon/Blueprints/Utils/BP_RoomManager.Spawn Traps` _output_get)
  (`self.K2_TeleportTo` (`GameplayStatics.GetPlayerCharacter` 0) (.location (`self.GetTransform` (`/Game/Dungeon/Blueprints/Utils/BP_RoomManager.PlayerSpawn` (`self.LastTrapRoom`)))) (.rotation (`self.GetTransform` (`/Game/Dungeon/Blueprints/Utils/BP_RoomManager.PlayerSpawn` (`self.LastTrapRoom`))))))

(fn `SpawnTrap`
  (params (SpawnTransformArray :type "Array of Transform Structure"))
  (locals (SpawnObject :type "Actor Class Reference") (ExcludeInd :type Integer))
  (if (`KismetMathLibrary.RandomBoolWithWeight` (`self.TrapSpawnChance`))
    (set `local.SpawnObject` (`KismetArrayLibrary.Array_Random` (`self.Traps`)))
    (else
      (set `local.SpawnObject` (`self.BaseFloor`))))
  (bind _output_get (set `local.ExcludeInd` (`.OutIndex` (`KismetArrayLibrary.Array_Random` SpawnTransformArray))))
  (`|SpawnActorFromClass` (`local.SpawnObject`) (`|GetArrayItem` SpawnTransformArray _output_get) "Undefined" "MultiplyWithRoot" null null)
  (for (_array_element _array_index) SpawnTransformArray
    (if (!= _array_index (`local.ExcludeInd`))
      (`|SpawnActorFromClass` (`self.BaseFloor`) _array_element "Undefined" "MultiplyWithRoot" null null))))

(fn `UserConstructionScript`)