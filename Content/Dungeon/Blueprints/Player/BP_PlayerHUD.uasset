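; BP_PlayerHUD is the dungeon game's canvas HUD, showing money, rooms completed and end-of-run messages.
; On BeginPlay it caches the player character and game mode by casting.
; Each DrawHUD polls the game mode's win and loss flags and draws text at fixed screen positions.
; A win replaces the stats with victory, final score and a restart prompt, while a loss adds a death message above the running stats.
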(event `self.ReceiveBeginPlay`
  (bind _asbp_player_character (cast `/Game/Dungeon/Blueprints/Player/BP_PlayerCharacter` (`GameplayStatics.GetPlayerCharacter` 0)))
  (set `self.PlayerRef` _asbp_player_character)
  (bind _asbp_game_mode (cast `/Game/Dungeon/Blueprints/Core/BP_GameMode` (`GameplayStatics.GetGameMode`)))
  (set `self.GameModeRef` _asbp_game_mode))

(event `self.ReceiveDrawHUD`
  (params (SizeX :type Integer) (SizeY :type Integer))
  (if (`/Game/Dungeon/Blueprints/Core/BP_GameMode.PlayerWon` (`self.GameModeRef`))
    (`self.DrawText` "Victory!" (struct :`G` 1.0 :`B` 0.025071 :`A` 1.0) 500.0 100.0 null 8.0)
    (`self.DrawText` (`KismetStringLibrary.BuildString_Int` "Final Score: " "" (`KismetMathLibrary.FTrunc` (`/Game/Dungeon/Blueprints/Player/BP_PlayerCharacter.Money` (`self.PlayerRef`)))) (struct :`R` 1.0 :`G` 0.814177 :`A` 1.0) 500.0 200.0 null 8.0)
    (`self.DrawText` "Press R to Restart" (struct :`G` 0.568019 :`B` 1.0 :`A` 1.0) 500.0 300.0 null 8.0)
    (else
      (if (`/Game/Dungeon/Blueprints/Core/BP_GameMode.PlayerLost` (`self.GameModeRef`))
        (`self.DrawText` "You Died" (struct :`R` 1.0 :`B` 0.005894 :`A` 1.0) 500.0 100.0 null 8.0))
      (`self.DrawText` (`KismetStringLibrary.BuildString_Int` "Money: " "" (`KismetMathLibrary.FTrunc` (`/Game/Dungeon/Blueprints/Player/BP_PlayerCharacter.Money` (`self.PlayerRef`)))) (struct :`R` 1.0 :`G` 0.814177 :`A` 1.0) 10.0 10.0 null 3.0)
      (`self.DrawText` (`KismetStringLibrary.BuildString_Int` "Rooms Completed: " "" (`/Game/Dungeon/Blueprints/Core/BP_GameMode.RoomsCompleted` (`self.GameModeRef`))) (struct :`G` 1.0 :`B` 0.061501 :`A` 1.0) 10.0 60.0 null 3.0))))

(fn `UserConstructionScript`)