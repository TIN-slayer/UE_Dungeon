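; BP_ButtonEscape is an interactable button that lets the player end a dungeon run early by escaping.
; On BeginPlay it binds to the game mode's safe-room-spawned event.
; Each time a safe room spawns, it shows its mesh and enables collision only if completed rooms meet the escape requirement, otherwise hiding and disabling itself.
; Interacting calls FinishTheRun on the game mode.
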(event `self.ReceiveBeginPlay`
  (`parent.ReceiveBeginPlay`)
  (add `/Game/Dungeon/Blueprints/Core/BP_GameMode.SafeRoomSpawned` (`self.GameModeRef`) (delegate `OnSafeRoomSpawn`)))

(event `OnSafeRoomSpawn`
  (if (>= (`/Game/Dungeon/Blueprints/Core/BP_GameMode.RoomsCompleted` (`self.GameModeRef`)) (`/Game/Dungeon/Blueprints/Core/BP_GameMode.TryToEscapeRoomReq` (`self.GameModeRef`)))
    (`PrimitiveComponent.SetCollisionEnabled` (`self.Box`) "QueryAndPhysics")
    (`SceneComponent.SetVisibility` (`self.StaticMesh`) true false)
    (else
      (`PrimitiveComponent.SetCollisionEnabled` (`self.Box`) "NoCollision")
      (`SceneComponent.SetVisibility` (`self.StaticMesh`) false false))))

(event `/Game/Dungeon/Blueprints/Interfaces/BPI_Interact.Interact`
  (`/Game/Dungeon/Blueprints/Core/BP_GameMode.FinishTheRun` (`self.GameModeRef`)))

(fn `UserConstructionScript`
  (`parent.UserConstructionScript`))