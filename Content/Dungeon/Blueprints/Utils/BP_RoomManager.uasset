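; Room manager actor for a dungeon that tracks a room's trap and player spawn points and controls trap spawning and cleanup.
; On BeginPlay it sorts the actors overlapping its Box into a trap spawn point list and a player spawn reference.
; SpawnTraps triggers each stored point.
; DestroyTraps removes all BP_BaseTrap and BP_Arrows actors in the whole world, not only those in this room.
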(event `self.ReceiveBeginPlay`
  (for _array_element (`PrimitiveComponent.GetOverlappingActors` (`self.Box`) null)
    (bind _asbp_trap_spawn_point (cast `/Game/Dungeon/Blueprints/Utils/BP_TrapSpawnPoint` _array_element)
      (:`then`
        (`KismetArrayLibrary.Array_Add` (`self.TrapSpawnPoints`) _asbp_trap_spawn_point))
      (:`CastFailed`
        (bind _asbp_player_spawn (cast `/Game/Dungeon/Blueprints/Utils/BP_PlayerSpawn` _array_element))
        (set `self.PlayerSpawn` _asbp_player_spawn)))))

(event `Spawn Traps`
  (for _array_element (`self.TrapSpawnPoints`)
    (`/Game/Dungeon/Blueprints/Utils/BP_TrapSpawnPoint.Spawn Trap` _array_element)))

(event `Destroy Traps`
  (bind _outactors (`GameplayStatics.GetAllActorsOfClass` "/Game/Dungeon/Blueprints/Traps/BP_BaseTrap.BP_BaseTrap_C"))
  (`self.K2_DestroyActor` _outactors)
  (bind _outactors_2 (`GameplayStatics.GetAllActorsOfClass` "/Game/Dungeon/Blueprints/Traps/TrapParts/BP_Arrows.BP_Arrows_C"))
  (`self.K2_DestroyActor` _outactors_2))

(fn `UserConstructionScript`)