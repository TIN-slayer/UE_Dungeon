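; Trap spawn point placed in generated dungeon rooms that finds nearby surfaces where traps can be mounted.
; On BeginPlay it line-traces along each enabled direction from a directions data table and records hits.
; AddSpawnPos maps each axis-aligned hit normal to a trap position and rotation, stored as transforms in a dictionary.
; SpawnTrap hands that dictionary and a second-floor flag to the game mode, which handles spawning.
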(event `self.ReceiveBeginPlay`
  (bind _spawndirections (`self.SpawnDirections`))
  (bind _returnvalue (`SceneComponent.K2_GetComponentLocation` (`self.DefaultSceneRoot`)))
  (bind _asbp_game_mode (cast `/Game/Dungeon/Blueprints/Core/BP_GameMode` (`GameplayStatics.GetGameMode`)))
  (set `self.GameMode` _asbp_game_mode)
  (bind _keys (`BlueprintMapLibrary.Map_Keys` _spawndirections))
  (for _array_element _keys
    (if (`BlueprintMapLibrary.Map_Find` _spawndirections _array_element)
      (bind _returnvalue_2 (`|GetDataTableRow` "/Game/Dungeon/Blueprints/Data/DT_Directions.DT_Directions" (`KismetStringLibrary.Conv_StringToName` _array_element))
        (:`then`
          (bind (_outhit _returnvalue_3) (`KismetSystemLibrary.LineTraceSingle` :`Start` _returnvalue :`End` (+ (* (`.DirectionVector_2_3DB7A8B540EA4CDEA08354A54B4F25B7` (break `/Game/Dungeon/Blueprints/Data/S_Directions` _returnvalue_2)) (`self.VectorDistance`)) _returnvalue) :`TraceChannel` "TraceTypeQuery1" :`DrawTime` 102.0))
          (if _returnvalue_3
            (bind (_bblockinghit _binitialoverlap _time _distance _location _impactpoint _normal) (`GameplayStatics.BreakHitResult` _outhit))
            (`self.AddSpawnPos` _location _normal)))))))

(event `Spawn Trap`
  (`/Game/Dungeon/Blueprints/Core/BP_GameMode.SpawnTrap` (`self.GameMode`) (`self.TrapSpawnsDict`) (`self.IsSecondFloor`)))

(fn `AddSpawnPos`
  (params (Location :type "Vector Structure") (Norm :type "Vector Structure"))
  (locals (X_Roll :type "Float (double-precision)") (Y_Pitch :type "Float (double-precision)") (Z_Yaw :type "Float (double-precision)") (TrapPosition :type "/Game/Dungeon/Blueprints/Utils/RoomGenerators/E_TrapPositions Enum"))
  (switch `string` (`KismetStringLibrary.Concat_StrStr` (`KismetStringLibrary.Conv_Int64ToString` (`KismetMathLibrary.Conv_DoubleToInt64` (.x Norm))) (`KismetStringLibrary.Conv_Int64ToString` (`KismetMathLibrary.Conv_DoubleToInt64` (.y Norm))) (`KismetStringLibrary.Conv_Int64ToString` (`KismetMathLibrary.Conv_DoubleToInt64` (.z Norm))))
    (:`001`
      (set `local.TrapPosition` "NewEnumerator2"))
    (:`00-1`
      (set `local.X_Roll` 180.0)
      (set `local.TrapPosition` "NewEnumerator1"))
    (:`010`
      (set `local.X_Roll` 90.0)
      (set `local.TrapPosition` "NewEnumerator5"))
    (:`0-10`
      (set `local.X_Roll` -90.0)
      (set `local.TrapPosition` "NewEnumerator6"))
    (:`100`
      (set `local.Y_Pitch` -90.0)
      (set `local.TrapPosition` "NewEnumerator3"))
    (:`-100`
      (set `local.Y_Pitch` 90.0)
      (set `local.TrapPosition` "NewEnumerator4")))
  (`BlueprintMapLibrary.Map_Add` (`self.TrapSpawnsDict`) (`local.TrapPosition`) (`KismetMathLibrary.MakeTransform` Location (`KismetMathLibrary.MakeRotator` (`local.X_Roll`) (`local.Y_Pitch`) (`local.Z_Yaw`)))))

(fn `UserConstructionScript`)