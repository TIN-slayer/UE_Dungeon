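; BP_BlessingText is a text render utility actor that shows the price of a blessing in the dungeon.
; On BeginPlay it casts the game mode to BP_GameMode and reads BlessingPrice.
; It appends that price as an integer and a "money" suffix to the TextRender component's existing text, once, with no later updates.
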(event `self.ReceiveBeginPlay`
  (bind _textrender (`self.TextRender`))
  (bind _asbp_game_mode (cast `/Game/Dungeon/Blueprints/Core/BP_GameMode` (`GameplayStatics.GetGameMode`)))
  (`TextRenderComponent.K2_SetText` _textrender (`KismetTextLibrary.Conv_StringToText` (`KismetStringLibrary.Concat_StrStr` (`KismetTextLibrary.Conv_TextToString` (`TextRenderComponent.Text` _textrender)) " " (`KismetStringLibrary.Conv_Int64ToString` (`KismetMathLibrary.Conv_DoubleToInt64` (`/Game/Dungeon/Blueprints/Core/BP_GameMode.BlessingPrice` _asbp_game_mode))) " money"))))

(fn `UserConstructionScript`)