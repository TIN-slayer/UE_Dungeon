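; Small spikes trap for the dungeon that damages the player on contact and moves its spikes as it pauses and unpauses.
; KillBox overlaps with the player character apply percentage-based damage, using the trap damage percent cached from BP_GameMode at BeginPlay.
; PauseTrap and UnpauseTrap slide the Spikes component to the StartPoint and ExitPoint relative locations respectively, over the lifting time.
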(event `self.ReceiveBeginPlay`
  (`parent.ReceiveBeginPlay`)
  (bind _asbp_game_mode (cast `/Game/Dungeon/Blueprints/Core/BP_GameMode` (`GameplayStatics.GetGameMode`)))
  (set `self.GameModeRef` _asbp_game_mode))

(event `self.KillBox.OnComponentBeginOverlap`
  (params (OverlappedComponent :type "PrimitiveComponent Object Reference") (OtherActor :type "Actor Object Reference") (OtherComp :type "PrimitiveComponent Object Reference") (OtherBodyIndex :type Integer) (bFromSweep :type Boolean) (SweepResult :type "HitResult Structure (by ref)"))
  (bind _asbp_player_character (cast `/Game/Dungeon/Blueprints/Player/BP_PlayerCharacter` OtherActor))
  (`/Game/Dungeon/Blueprints/Player/BP_PlayerCharacter.ApplyDamage` _asbp_player_character 0.0 (`/Game/Dungeon/Blueprints/Core/BP_GameMode.TrapDamagePercent` (`self.GameModeRef`))))

(event `self.PauseTrap`
  (`KismetSystemLibrary.MoveComponentTo` (`self.Spikes`) (`SceneComponent.RelativeLocation` (`self.StartPoint`)) (struct) false false (`self.SpikesLiftingTime`)))

(event `self.UnpauseTrap`
  (`KismetSystemLibrary.MoveComponentTo` (`self.Spikes`) (`SceneComponent.RelativeLocation` (`self.ExitPoint`)) (struct) false false (`self.SpikesLiftingTime`)))

(fn `UserConstructionScript`
  (`parent.UserConstructionScript`))