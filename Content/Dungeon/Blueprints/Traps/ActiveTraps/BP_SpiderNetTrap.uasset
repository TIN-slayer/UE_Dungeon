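; BP_SpiderNetTrap is a dungeon spider net trap that slows the player character while inside its SlowBox.
; On overlap begin it multiplies the character's max walk speed by SpeedDebuff, and on overlap end divides it back, both based on GetMaxSpeed rather than a cached original.
; A DestroySpderNet event removes both the SlowBox and SpiderNet components, leaving the actor itself in place.
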(event `self.SlowBox.OnComponentBeginOverlap`
  (params (OverlappedComponent :type "PrimitiveComponent Object Reference") (OtherActor :type "Actor Object Reference") (OtherComp :type "PrimitiveComponent Object Reference") (OtherBodyIndex :type Integer) (bFromSweep :type Boolean) (SweepResult :type "HitResult Structure (by ref)"))
  (bind _asbp_player_character (cast `/Game/Dungeon/Blueprints/Player/BP_PlayerCharacter` OtherActor))
  (bind _charactermovement (`Character.CharacterMovement` _asbp_player_character))
  (set `CharacterMovementComponent.MaxWalkSpeed` (* (`MovementComponent.GetMaxSpeed` _charactermovement) (`self.SpeedDebuff`)) _charactermovement))

(event `self.SlowBox.OnComponentEndOverlap`
  (params (OverlappedComponent :type "PrimitiveComponent Object Reference") (OtherActor :type "Actor Object Reference") (OtherComp :type "PrimitiveComponent Object Reference") (OtherBodyIndex :type Integer))
  (bind _asbp_player_character (cast `/Game/Dungeon/Blueprints/Player/BP_PlayerCharacter` OtherActor))
  (bind _charactermovement (`Character.CharacterMovement` _asbp_player_character))
  (set `CharacterMovementComponent.MaxWalkSpeed` (/ (`MovementComponent.GetMaxSpeed` _charactermovement) (`self.SpeedDebuff`)) _charactermovement))

(event `DestroySpderNet`
  (`ActorComponent.K2_DestroyComponent` (`self.SlowBox`))
  (`ActorComponent.K2_DestroyComponent` (`self.SpiderNet`)))

(fn `UserConstructionScript`
  (`parent.UserConstructionScript`))