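; BP_ArrowsTrap is an active dungeon trap that fires arrows at a regular interval.
; On BeginPlay it starts a looping timer at DelayTime, with a random initial start delay up to MaxStartDelayTime.
; Each Fire call spawns a BP_Arrows actor at the ExitPoint location, oriented to the Platform's world rotation.
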(event `self.ReceiveBeginPlay`
  (`KismetSystemLibrary.K2_SetTimer` null "Fire" (`self.DelayTime`) true false (`KismetMathLibrary.RandomFloatInRange` 0.0 (`self.MaxStartDelayTime`))))

(event `Fire`
  (`|SpawnActorFromClass` "/Game/Dungeon/Blueprints/Traps/TrapParts/BP_Arrows.BP_Arrows_C" (`KismetMathLibrary.MakeTransform` (`SceneComponent.K2_GetComponentLocation` (`self.ExitPoint`)) (`SceneComponent.K2_GetComponentRotation` (`self.Platform`))) "Undefined" "MultiplyWithRoot" null null))

(fn `UserConstructionScript`
  (`parent.UserConstructionScript`))