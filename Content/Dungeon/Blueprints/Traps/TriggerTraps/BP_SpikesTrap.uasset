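; BP_SpikesTrap is a triggered dungeon trap whose spikes extend on activation and then retract.
; ActivateTrap waits a configurable delay, slides the Spikes component to the ExitPoint, holds it up, then calls DeactivateTrap to move it back to StartPoint.
; A KillBox overlap detects the third-person character but only prints "DEAD" rather than applying damage.
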(event `self.Activate Trap`
  (`KismetSystemLibrary.Delay` (`self.DelayTime`))
  (`KismetSystemLibrary.MoveComponentTo` (`self.Spikes`) (`SceneComponent.RelativeLocation` (`self.ExitPoint`)) (struct) false false (`self.ActivatingTime`))
  (`KismetSystemLibrary.Delay` (`self.StayingUpTime`))
  (`self.Deactivate Trap`))

(event `self.Deactivate Trap`
  (`KismetSystemLibrary.MoveComponentTo` (`self.Spikes`) (`SceneComponent.RelativeLocation` (`self.StartPoint`)) (struct) false false (`self.DeactivatingTime`)))

(event `self.KillBox.OnComponentBeginOverlap`
  (params (OverlappedComponent :type "PrimitiveComponent Object Reference") (OtherActor :type "Actor Object Reference") (OtherComp :type "PrimitiveComponent Object Reference") (OtherBodyIndex :type Integer) (bFromSweep :type Boolean) (SweepResult :type "HitResult Structure (by ref)"))
  (cast `/Game/Dungeon/Blueprints/Player/BP_ThirdPersonCharacter` OtherActor)
  (`KismetSystemLibrary.PrintString` "DEAD"))

(fn `UserConstructionScript`
  (`parent.UserConstructionScript`))